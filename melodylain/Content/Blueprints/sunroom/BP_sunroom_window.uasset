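; Sunroom window actor that the player can break once enough hammers have been collected.
; Collecting a hammer increments a counter, copies it to the tank-controls character and adds a hammer HUD widget to the viewport.
; On Interact with the required count, it plays a glass sound, removes the widget, disables window collision and swaps the intact mesh for the initially hidden broken one.
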(event Custom|collectHammer
  ;[1 1 1] inc hammer
  (bind _result (Math|Integer|IncrementInt (Variables|Default|GethammerCollected))
    (:%20%20
      ;[1 1 1] add to viewport
      (bind _asbp_tank_controls_character (Utilities|Casting|CastToBP_TankControlsCharacter (Game|GetPlayerCharacter 0)))
      (Variables|/Game/Blueprints/character/BP_TankControlsCharacter.BP_TankControlsCharacter_C|SethammerSunroom _asbp_tank_controls_character _result)
      (bind _returnvalue (UserInterface|CreateWidget "/Game/Blueprints/widgets/HUD_hammer.HUD_hammer_C" (Game|GetPlayerController 0)))
      (bind _output_get (Variables|Default|SethudWidget _returnvalue))
      (UserInterface|Viewport|AddtoViewport _output_get 0))))

(event EventBeginPlay
  ;[1 1 1] broken window invisible
  (Rendering|SetVisibility (Variables|Default|Getsunroom_windowBroken) false false))

(event EventInteract
  ;[1 1 1] break glass
  (if (>= (Variables|Default|GethammerCollected) (Variables|Default|GetmaxHammers))
    (Audio|PlaySound2D "/Game/music/sfx/glass.glass" 1.0 1.0 0.0 0 0)
    (Variables|Default|SetwindowBroke? true)
    ;[1 1 1] remove from viewport
    (Utilities|Casting|CastToBP_TankControlsCharacter (Game|GetPlayerCharacter 0))
    (Widget|RemovefromParent (Variables|Default|GethudWidget))
    (Rendering|SetVisibility (Variables|Default|Getwindow) false false)
    (Rendering|SetVisibility (Variables|Default|Getsunroom_windowBroken) true false)
    (Collision|SetCollisionEnabled (Variables|Default|Getwindow) "NoCollision")))

(fn ConstructionScript)