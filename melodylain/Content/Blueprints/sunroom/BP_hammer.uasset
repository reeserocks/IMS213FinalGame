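; BP_hammer is a hammer pickup in the sunroom that reports its collection to the sunroom window.
; Any overlap with its sphere plays a pickup sound, calls CollectHammer on the BP_sunroom_window found via GetActorOfClass, then destroys the hammer.
; From BeginPlay, a timeline continuously swings the hammer mesh's yaw back and forth by alternating Play and Reverse each time it finishes.
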(event OnComponentBeginOverlap(sphere_0)
  (params (OverlappedComponent :type Primitive%20Component%20Object%20Reference) (OtherActor :type Actor%20Object%20Reference) (OtherComp :type Primitive%20Component%20Object%20Reference) (OtherBodyIndex :type Integer) (bFromSweep :type Boolean) (SweepResult :type Hit%20Result%20Structure%20%28by%20ref%29))
  ;[1 1 1] collect item
  (Audio|PlaySound2D "/Game/music/sfx/pickUp.pickUp" 1.0 1.0 0.0 0 0)
  (bind _returnvalue (Actor|GetActorOfClass "/Game/Blueprints/sunroom/BP_sunroom_window.BP_sunroom_window_C"))
  (Default|CollectHammer _returnvalue)
  (Actor|DestroyActor))

(event Custom|anim
  ;[1 1 1] animation
  (bind (_direction _offsetalpha) (Timeline|rotateHammer Play)
    (:Update
      (Transformation|SetRelativeRotation (Variables|Default|Gethammer) (Math|Rotator|MakeRotator 0.0 0.0 (* _offsetalpha (Variables|Default|Getrotation))) false false))
    (:Finished
      (switch Utilities|FlowControl|Switch|SwitchonETimelineDirection _direction
        (:Forward
          (CallFunction|ReverseAnim))
        (:Backward
          (CallFunction|Anim))))))

(event Custom|reverse%20anim
  ;[1 1 1] animation
  (bind (_direction _offsetalpha) (Timeline|rotateHammer Reverse)
    (:Update
      (Transformation|SetRelativeRotation (Variables|Default|Gethammer) (Math|Rotator|MakeRotator 0.0 0.0 (* _offsetalpha (Variables|Default|Getrotation))) false false))
    (:Finished
      (switch Utilities|FlowControl|Switch|SwitchonETimelineDirection _direction
        (:Forward
          (CallFunction|ReverseAnim))
        (:Backward
          (CallFunction|Anim))))))

(event EventBeginPlay
  ;[1 1 1] play anim
  (CallFunction|Anim))

(fn ConstructionScript)