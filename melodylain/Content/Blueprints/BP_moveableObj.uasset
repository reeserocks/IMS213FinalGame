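; Pushable sunroom chair that the tank-controls player character can shove.
; Two trigger volumes, one for the X axis and one for Y, detect the character's overlap.
; On begin overlap the chair starts simulating physics and the character's IsPushing flag is set; on end overlap both are switched off.
; Both axes run identical logic, with no axis-specific constraint in the graph.
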(event OnComponentBeginOverlap(y-axiscollision)
  (params (OverlappedComponent :type Primitive%20Component%20Object%20Reference) (OtherActor :type Actor%20Object%20Reference) (OtherComp :type Primitive%20Component%20Object%20Reference) (OtherBodyIndex :type Integer) (bFromSweep :type Boolean) (SweepResult :type Hit%20Result%20Structure%20%28by%20ref%29))
  ;[1 1 1] pushing y
  (bind _asbp_tank_controls_character (Utilities|Casting|CastToBP_TankControlsCharacter OtherActor))
  (Physics|SetSimulatePhysics (Variables|Default|Getsunroom_chair) true)
  (Variables|/Game/Blueprints/character/BP_TankControlsCharacter.BP_TankControlsCharacter_C|SetisPushing? _asbp_tank_controls_character true))

(event OnComponentEndOverlap(y-axiscollision)
  (params (OverlappedComponent :type Primitive%20Component%20Object%20Reference) (OtherActor :type Actor%20Object%20Reference) (OtherComp :type Primitive%20Component%20Object%20Reference) (OtherBodyIndex :type Integer))
  ;[1 1 1] not pushing y
  (bind _asbp_tank_controls_character (Utilities|Casting|CastToBP_TankControlsCharacter OtherActor))
  (Physics|SetSimulatePhysics (Variables|Default|Getsunroom_chair) false)
  (Variables|/Game/Blueprints/character/BP_TankControlsCharacter.BP_TankControlsCharacter_C|SetisPushing? _asbp_tank_controls_character false))

(event OnComponentBeginOverlap(x-asiscollision)
  (params (OverlappedComponent :type Primitive%20Component%20Object%20Reference) (OtherActor :type Actor%20Object%20Reference) (OtherComp :type Primitive%20Component%20Object%20Reference) (OtherBodyIndex :type Integer) (bFromSweep :type Boolean) (SweepResult :type Hit%20Result%20Structure%20%28by%20ref%29))
  ;[1 1 1] pushing x
  (bind _asbp_tank_controls_character (Utilities|Casting|CastToBP_TankControlsCharacter OtherActor))
  (Physics|SetSimulatePhysics (Variables|Default|Getsunroom_chair) true)
  (Variables|/Game/Blueprints/character/BP_TankControlsCharacter.BP_TankControlsCharacter_C|SetisPushing? _asbp_tank_controls_character true))

(event OnComponentEndOverlap(x-asiscollision)
  (params (OverlappedComponent :type Primitive%20Component%20Object%20Reference) (OtherActor :type Actor%20Object%20Reference) (OtherComp :type Primitive%20Component%20Object%20Reference) (OtherBodyIndex :type Integer))
  ;[1 1 1] not pushing x
  (bind _asbp_tank_controls_character (Utilities|Casting|CastToBP_TankControlsCharacter OtherActor))
  (Physics|SetSimulatePhysics (Variables|Default|Getsunroom_chair) false)
  (Variables|/Game/Blueprints/character/BP_TankControlsCharacter.BP_TankControlsCharacter_C|SetisPushing? _asbp_tank_controls_character false))

(fn ConstructionScript)