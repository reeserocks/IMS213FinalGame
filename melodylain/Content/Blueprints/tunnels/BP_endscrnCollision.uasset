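; BP_endscrnCollision is an interactable in the tunnels area that ends play with a story end screen.
; Its Interact event pauses the game, shows the mouse cursor and switches input to UI only.
; It then increments NumGhosts on the BP_TankControlsCharacter player, creates the Endscrn_story widget and adds it to the viewport.
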(event EventInteract
  (bind _returnvalue (Game|GetPlayerController 0))
  (Game|SetGamePaused true)
  (Variables|/Script/Engine.PlayerController|SetbShowMouseCursor _returnvalue true)
  (Input|SetInputModeUIOnly _returnvalue 0 "DoNotLock" false)
  (bind _asbp_tank_controls_character (Utilities|Casting|CastToBP_TankControlsCharacter (Game|GetPlayerCharacter 0)))
  (Variables|/Game/Blueprints/character/BP_TankControlsCharacter.BP_TankControlsCharacter_C|SetnumGhosts _asbp_tank_controls_character (+ (Variables|/Game/Blueprints/character/BP_TankControlsCharacter.BP_TankControlsCharacter_C|GetnumGhosts _asbp_tank_controls_character) 1))
  (bind _returnvalue_2 (UserInterface|CreateWidget "/Game/Blueprints/widgets/endscrn_story.endscrn_story_C" (Game|GetPlayerController 0)))
  (bind _output_get (Variables|Default|Setendscrn _returnvalue_2))
  (UserInterface|Viewport|AddtoViewport _output_get 0))

(fn ConstructionScript)