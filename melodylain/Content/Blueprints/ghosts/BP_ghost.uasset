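; BP_ghost is a collectible ghost that spins in place and is given relative InterpToMovement points for vertical bobbing.
; Any actor overlap increments NumGhosts on the player's BP_TankControlsCharacter, without checking which actor overlapped.
; It then pauses the game, shows the GhostBasic widget with mouse cursor and UI-only input, and destroys itself.
; Tick applies yaw scaled by delta time, while the construction script adds the movement control points.
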(event EventTick
  (params (DeltaSeconds :type Float%20%28single-precision%29))
  ;[1 1 1] rotate ghosty
  (Transformation|AddActorLocalRotation (Math|Rotator|MakeRotator 0.0 0.0 (* DeltaSeconds (Variables|Default|Getrotation))) false false))

(event Collision|EventActorBeginOverlap
  (params (OtherActor :type Actor%20Object%20Reference))
  (bind _returnvalue (Game|GetPlayerController 0))
  ;[1 1 1] add to hud
  (bind _asbp_tank_controls_character (Utilities|Casting|CastToBP_TankControlsCharacter (Game|GetPlayerCharacter 0)))
  (Variables|/Game/Blueprints/character/BP_TankControlsCharacter.BP_TankControlsCharacter_C|SetnumGhosts _asbp_tank_controls_character (+ (Variables|/Game/Blueprints/character/BP_TankControlsCharacter.BP_TankControlsCharacter_C|GetnumGhosts _asbp_tank_controls_character) 1))
  (Game|SetGamePaused true)
  (bind _returnvalue_2 (UserInterface|CreateWidget "/Game/Blueprints/widgets/ghost/ghostBasic.ghostBasic_C" (Game|GetPlayerController 0)))
  (bind _output_get (Variables|Default|SetghostWidget _returnvalue_2))
  (UserInterface|Viewport|AddtoViewport _output_get 0)
  (Variables|/Script/Engine.PlayerController|SetbShowMouseCursor _returnvalue true)
  (Input|SetInputModeUIOnly _returnvalue (Variables|Default|GetghostWidget) "DoNotLock" false)
  (Actor|DestroyActor))

(fn ConstructionScript
  (Class|InterptoMovementComponent|AddControlPointPosition (Variables|Default|GetInterpToMovement) "0, 0, 0" true)
  (Class|InterptoMovementComponent|AddControlPointPosition (Variables|Default|GetInterpToMovement) "0.000000,0.000000,30.000000" true))