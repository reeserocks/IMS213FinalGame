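; Bedroom door that opens once the player has collected enough keys.
; Collecting a key increments the door's count, copies it to the tank-controls character and adds a key widget to the HUD.
; Interacting with enough keys plays a sound, triggers the door-opening update and spends a key, once only, with a timeline defining the yaw swing.
; While the door is open, Tick removes the key widget every frame.
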(event Custom|openDoor
  ;[1 1 1] open door anim
  (bind _door_rotation (Timeline|open%20door%20anim Play)
    (:Update
      (Transformation|SetRelativeRotation (Variables|Default|Getfixed_door1) (Math|Rotator|MakeRotator 0.0 0.0 (Math|Float|Lerp 0.0 1e+02 _door_rotation)) false false))))

(event Custom|collectItem
  ;[1 1 1] add key to inventory
  (bind _result (Math|Integer|IncrementInt (Variables|Default|GetkeysCollected))
    (:%20%20
      ;[1 1 1] show on HUD
      (bind _asbp_tank_controls_character (Utilities|Casting|CastToBP_TankControlsCharacter (Game|GetPlayerCharacter 0)))
      (Variables|/Game/Blueprints/character/BP_TankControlsCharacter.BP_TankControlsCharacter_C|SetkeyBedroom _asbp_tank_controls_character _result)
      (bind _returnvalue (UserInterface|CreateWidget "/Game/Blueprints/widgets/HUD_key.HUD_key_C" (Game|GetPlayerController 0)))
      (bind _output_get (Variables|Default|SetHUD_widget _returnvalue))
      (UserInterface|Viewport|AddtoViewport _output_get 0))))

(event EventTick
  (params (DeltaSeconds :type Float%20%28single-precision%29))
  (if (Variables|Default|GetdoorOpen?)
    (Utilities|Casting|CastToBP_TankControlsCharacter (Game|GetPlayerCharacter 0))
    (Widget|RemovefromParent (Variables|Default|GetHUD_widget))))

(event EventInteract
  (if (>= (Variables|Default|GetkeysCollected) (Variables|Default|GetmaxKeys))
    (Utilities|FlowControl|DoOnce false
      (:Completed
        (Audio|PlaySound2D "/Game/music/sfx/door.door" 1.0 1.0 0.0 0 0)
        (CallFunction|OpenDoorAnimUpdateFunc)
        (Variables|Default|SetdoorOpen? true)
        (Math|Integer|DecrementInt (Variables|Default|GetkeysCollected))))))

(fn ConstructionScript)